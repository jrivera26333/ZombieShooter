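; Behavior tree task that sends an AI-controlled pawn toward a location read from a blackboard key.
; It starts a simple move, then, for a BP_ZombieCharacter within 50 units of its TargetPosition, calls GetRandomPosition on it.
; For a zombie it finishes successfully right away without waiting for arrival; a failed cast never finishes the task.
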(event EventReceiveExecuteAI
  (params (OwnerController :type AI%20Controller%20Object%20Reference) (ControlledPawn :type Pawn%20Object%20Reference))
  (AI|Navigation|SimpleMovetoLocation OwnerController (Class|BTFunctionLibrary|GetBlackboardValueasVector (Variables|Default|GetBB_Ref)))
  (bind _asbp_zombie_character (Utilities|Casting|CastToBP_ZombieCharacter ControlledPawn))
  (if (<= (Math|Vector|Distance(Vector) (Transformation|GetActorLocation _asbp_zombie_character) (Variables|/Game/Blueprints/AI/BP_ZombieCharacter.BP_ZombieCharacter_C|GetTargetPosition _asbp_zombie_character)) 5e+01)
    (Default|GetRandomPosition _asbp_zombie_character))
  (AI|BehaviorTree|FinishExecute true))