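; Main player controller for an ALS (Advanced Locomotion System) character, handling the debug HUD and overlay state selection UI.
; On BeginPlay, the local controller adds the ALS HUD only if the possessed character has a debug component.
; Holding OpenOverlayMenu shows a switcher widget that the cycle inputs step through, and releasing it applies the selection.
; Menu slow motion is inactive, as its branches never run and the time dilation function is empty.
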(event EventBeginPlay
  (bind _possessedcharacter (Variables|Default|GetPossessedCharacter))
  (if (Pawn|IsLocalController)
    ;[1 1 1] Create and add HUD to Viewport if debug component exists in character
    (Utilities|IsValid _possessedcharacter
      (:Is%20Valid
        (Utilities|IsValid (Actor|GetComponentbyClass _possessedcharacter "/Script/ALSV4_CPP.ALSDebugComponent")
          (:Is%20Valid
            (bind _returnvalue (UserInterface|CreateWidget "/ALSV4_CPP/AdvancedLocomotionV4/Blueprints/UI/ALS_HUD.ALS_HUD_C" self))
            (bind _output_get (Variables|Default|SetBM_HUD _returnvalue))
            (UserInterface|Viewport|AddtoViewport _output_get 0)
            (Input|SetInputModeGameOnly self)))))))

(event Input|ActionEvents|InputActionOpenOverlayMenu
  (params (Key :type Key%20Structure :default "None"))
  ;[1 1 1] Switch Overlay States
  (:Pressed
    (Variables|Default|SetOverlayMenuOpen true)
    (if true
      _
      (else
        (CallFunction|SetGlobalTimeDilationLocal 0.35)))
    (bind _returnvalue (UserInterface|CreateWidget "/ALSV4_CPP/AdvancedLocomotionV4/Blueprints/UI/OverlayStateSwitcher.OverlayStateSwitcher_C" self))
    (bind _output_get (Variables|Default|SetOverlaySwitcher _returnvalue))
    (UserInterface|Viewport|AddtoViewport _output_get 0)
    (Audio|PlaySound2D "/ALSV4_CPP/AdvancedLocomotionV4/Audio/UI/Click.Click" 1.25 1.0 0.2 0 0))
  (:Released
    (Variables|Default|SetOverlayMenuOpen false)
    (if true
      _
      (else
        (CallFunction|SetGlobalTimeDilationLocal 1.0)))
    (Default|SelectOverlayState (Variables|Default|GetOverlaySwitcher))
    (Widget|RemovefromParent (Variables|Default|GetOverlaySwitcher))
    (Audio|PlaySound2D "/ALSV4_CPP/AdvancedLocomotionV4/Audio/UI/Click.Click" 1.25 1.0 0.2 0 0)))

(event Input|ActionEvents|InputActionCycleOverlayUp
  (params (Key :type Key%20Structure :default "None"))
  ;[1 1 1] Switch Overlay States
  (:Pressed
    (if (Variables|Default|GetOverlayMenuOpen)
      (bind _overlayswitcher (Variables|Default|GetOverlaySwitcher)
        (:then
          (Default|CycleState _overlayswitcher true)
          (Audio|PlaySound2D "/ALSV4_CPP/AdvancedLocomotionV4/Audio/UI/Click.Click" 1.25 1.0 0.2 0 0))
        (:else)))))

(event Input|ActionEvents|InputActionCycleOverlayDown
  (params (Key :type Key%20Structure :default "None"))
  ;[1 1 1] Switch Overlay States
  (:Pressed
    (if (Variables|Default|GetOverlayMenuOpen)
      (bind _overlayswitcher (Variables|Default|GetOverlaySwitcher)
        (:then
          (Default|CycleState _overlayswitcher false)
          (Audio|PlaySound2D "/ALSV4_CPP/AdvancedLocomotionV4/Audio/UI/Click.Click" 1.25 1.0 0.2 0 0))
        (:else)))))

(fn ConstructionScript)

(fn SetGlobalTimeDilationLocal
  (params (Dilation :type Float%20%28single-precision%29)))