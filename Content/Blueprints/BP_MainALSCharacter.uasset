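; Advanced Locomotion System character Blueprint that adds rifle ammo, firing and reloading.
; Interface events from notifies and montages update weapon state and ammo; reload plays a montage unless the state blocks it.
; Fire and reload montages are chosen by overlay state, with only Rifle supplying animations.
; Firing is unwired: FireEvent and GetEndLineTrace are empty, leaving the muzzle-socket trace that ragdolls hit characters unreachable.
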(event EventBPIonFiring
  ;[1 1 1] Called within Notifies
  (CallFunction|FireEvent))

(event EventBPISetWeaponState
  (params (State :type WeaponState%20Enum :default "NewEnumerator0"))
  ;[1 1 1] Keeping track of state to prevent weapon reload overlapping
  (Variables|Default|SetWeaponState State))

(event EventBPISetAmmo
  (params (AmountOfAmmo :type Integer))
  ;[1 1 1] In the montage we are updating the ammo count
  (Variables|Default|SetAmmo AmountOfAmmo)
  (CallFunction|FireEvent))

(event Custom|Reload%20Event
  ;[0.4476 0.2572 1] Reloading Event/Action
  (if (Utilities|Enum|NotEqual(Enum) (Variables|Default|GetWeaponState) "NewEnumerator1")
    (bind _returnvalue (Class|ALSBaseCharacter|GetMainAnimInstance))
    (Utilities|IsValid _returnvalue
      (:Is%20Valid
        (Animation|Montage|MontagePlay _returnvalue (CallFunction|GetReloadAnimation) 1.0 "MontageLength" 0.0 true))
      (:Is%20Not%20Valid
        (Development|PrintString "Could not find Anim Instance")))))

(event Custom|Fire%20Event
  ;[1 0.01042 0.01042] Fire Event/Action
)

(event Input|ActionEvents|InputActionReloadAction
  (params (Key :type Key%20Structure :default "None"))
  ;[0.4476 0.2572 1] Reloading Event/Action
)

(event Input|ActionEvents|InputActionFire
  (params (Key :type Key%20Structure :default "None"))
  ;[1 0.01042 0.01042] Fire Event/Action
)

(fn ConstructionScript
  (|CallParentFunction))

(fn GetFireAnimation
  (bind _overlaystate (Variables|Default|GetOverlayState))
  (Development|PrintString (Utilities|String|EnumtoString _overlaystate))
  (switch Utilities|FlowControl|Switch|SwitchonEALSOverlayState _overlaystate
    (:Default
      _)
    (:Masculine
      _)
    (:Feminine
      _)
    (:Injured
      _)
    (:HandsTied
      _)
    (:Rifle
      (Development|PrintString "FIRED")
      (return (Variables|Default|GetFireAnimation)))
    (:PistolOneHanded
      _)
    (:PistolTwoHanded
      _)
    (:Bow
      _)
    (:Torch
      _)
    (:Binoculars
      _)
    (:Box
      _)
    (:Barrel
      _))
  (return 0))

(fn GetReloadAnimation
  (bind _overlaystate (Variables|Default|GetOverlayState))
  (Development|PrintString (Utilities|String|EnumtoString _overlaystate))
  (switch Utilities|FlowControl|Switch|SwitchonEALSOverlayState _overlaystate
    (:Default
      _)
    (:Masculine
      _)
    (:Feminine
      _)
    (:Injured
      _)
    (:HandsTied
      _)
    (:Rifle
      (return (Variables|Default|GetReloadAnimation)))
    (:PistolOneHanded
      _)
    (:PistolTwoHanded
      _)
    (:Bow
      _)
    (:Torch
      _)
    (:Binoculars
      _)
    (:Box
      _)
    (:Barrel
      _))
  (return 0))

(fn GetEndLineTrace
  (params (self2 :type Scene%20Component%20Object%20Reference)))

(fn BPIGetAmmo
  (return (Variables|Default|GetAmmo)))